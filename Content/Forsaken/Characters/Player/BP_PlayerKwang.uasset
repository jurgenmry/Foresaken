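; Player character Blueprint for Kwang, with control-yaw-relative movement, a melee combo and two abilities.
; Attack input plays four montages in sequence, briefly locking movement and buffering presses made mid-swing until ComboAttackSave continues the chain or ResetCombo clears it.
; GroundHit and Dash delegate to BPCAbilities, while a sphere tracks overlapping BPI_Abilities actors during an active ground pound.
; BeginPlay initializes health and damage and shows the cursor, but mouse-facing rotation is disconnected.
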(event `InputAxis|Turn Right / Left Gamepad`
  (params (AxisValue :type "Float (single-precision)"))
  ;[1 0 0] MOVEMENT
  ;;[1 1 1] Gamepad input // DEFAULT
  (`self.AddControllerYawInput` AxisValue))

(event `InputAxis|Move Forward / Backward`
  (params (AxisValue :type "Float (single-precision)"))
  ;[1 0 0] MOVEMENT
  ;;[1 1 1] Movement input // DEFAULT
  (`self.AddMovementInput` (`KismetMathLibrary.GetForwardVector` (`KismetMathLibrary.MakeRotator` 0.0 0.0 (.yaw (`self.GetControlRotation`)))) AxisValue))

(event `InputAxis|Look Up / Down Mouse`
  (params (AxisValue :type "Float (single-precision)"))
  ;[1 0 0] MOVEMENT
  ;;[1 1 1] Mouse input // DEFAULT
)

(event `InputAxis|Look Up / Down Gamepad`
  (params (AxisValue :type "Float (single-precision)"))
  ;[1 0 0] MOVEMENT
  ;;[1 1 1] Gamepad input // DEFAULT
  (`self.AddControllerPitchInput` (* AxisValue (`self.BaseLookUpRate`) (`GameplayStatics.GetWorldDeltaSeconds`))))

(event `InputAction|Jump` :overrideparent false
  (params (Key :type "Key Structure"))
  ;[1 0 0] MOVEMENT
  ;;[1 1 1] Jump // DEFAULT
)

(event `InputAxis|Move Right / Left`
  (params (AxisValue :type "Float (single-precision)"))
  ;[1 0 0] MOVEMENT
  ;;[1 1 1] Movement input // DEFAULT
  (`self.AddMovementInput` (`KismetMathLibrary.GetRightVector` (`KismetMathLibrary.MakeRotator` 0.0 0.0 (.yaw (`self.GetControlRotation`)))) AxisValue))

(event `self.ReceiveTick`
  (params (DeltaSeconds :type "Float (single-precision)"))
  ;[1 0 0] MOVEMENT
  ;;[0 1 0] Mouse Rotation
)

(event `self.ReceiveBeginPlay`
  (bind _bpc_health (`self.BPC_Health`))
  ;[1 0 0] Begin Play
  (set `PlayerController.bShowMouseCursor` true (`GameplayStatics.GetPlayerController` 0))
  (bind _output_get (set `/Game/Forsaken/Characters/BPC_Health.HealthMax` (`self.HealthMax`) _bpc_health))
  (set `/Game/Forsaken/Characters/BPC_Health.CurrentHealth` _output_get _bpc_health)
  (`KismetSystemLibrary.PrintString` (`KismetStringLibrary.Conv_DoubleToString` (`/Game/Forsaken/Characters/BPC_Health.HealthMax` _bpc_health)) true true (struct :`G` 0.66 :`B` 1.0 :`A` 1.0) 3.0)
  (bind _output_get_2 (set `self.DamageCurrent` (`self.DamageBase`)))
  (`KismetSystemLibrary.PrintString` (`KismetStringLibrary.Conv_DoubleToString` _output_get_2) true true (struct :`G` 0.66 :`B` 1.0 :`A` 1.0) 3.0))

(event `InputAction|Attack`
  (params (Key :type "Key Structure"))
  (bind _charactermovement (`self.CharacterMovement`))
  ;[0 1 0] Combo System Setup.
  (:`Pressed`
    (if (`self.IsAttacking`)
      (set `self.SaveAttack` true)
      (else
        (set `self.IsAttacking` true)
        (switch `int` (`self.AttackCount`) :!label _label
          (:`0`
            (set `self.AttackCount` 1)
            (`|PlayMontage` (`self.Mesh`) "/Game/Forsaken/Characters/Player/PrimaryAttack_A_Montage.PrimaryAttack_A_Montage" 1.8 0.05
              (:`then`
                _)))
          (:`1`
            (set `self.AttackCount` 2)
            (`|PlayMontage` (`self.Mesh`) "/Game/Forsaken/Characters/Player/PrimaryAttack_B_Montage.PrimaryAttack_B_Montage" 1.8 0.05
              (:`then`
                _)))
          (:`2`
            (set `self.AttackCount` 3)
            (`|PlayMontage` (`self.Mesh`) "/Game/Forsaken/Characters/Player/PrimaryAttack_C_Montage.PrimaryAttack_C_Montage" 1.8 0.05
              (:`then`
                _)))
          (:`3`
            (set `self.AttackCount` 0)
            (`|PlayMontage` (`self.Mesh`) "/Game/Forsaken/Characters/Player/PrimaryAttack_D_Montage.PrimaryAttack_D_Montage" 1.8 0.05
              (:`then`
                _))))
        (`CharacterMovementComponent.DisableMovement` _charactermovement)
        (`KismetSystemLibrary.Delay` 0.45)
        (`CharacterMovementComponent.SetMovementMode` _charactermovement "MOVE_Walking" 0)))))

(event `ComboAttackSave`
  ;[0 1 0] Combo System Setup.
  (if (`self.SaveAttack`)
    (set `self.SaveAttack` false)
    (goto _label)))

(event `ResetCombo`
  ;[0 1 0] Combo System Setup.
  (set `self.AttackCount` 0)
  (set `self.SaveAttack` false)
  (set `self.IsAttacking` false))

(event `InputAction|GroundHit`
  (params (Key :type "Key Structure"))
  ;[0 1 0] GROUND HIT ABILITY
  (:`Pressed`
    (`/Game/Forsaken/Characters/BPC_Abilities.GroundHit` (`self.BPC_Abilities`) (`self.Ground Hit Cooldown`))))

(event `InputAction|Dash`
  (params (Key :type "Key Structure"))
  ;[0 1 0] DASH ABILITY
  (:`Pressed`
    (`/Game/Forsaken/Characters/BPC_Abilities.Dash` (`self.BPC_Abilities`) (`self.DashCooldown`))))

(event `self.Sphere.OnComponentBeginOverlap`
  (params (OverlappedComponent :type "PrimitiveComponent Object Reference") (OtherActor :type "Actor Object Reference") (OtherComp :type "PrimitiveComponent Object Reference") (OtherBodyIndex :type Integer) (bFromSweep :type Boolean) (SweepResult :type "HitResult Structure (by ref)"))
  ;[1 0.5 0] Store Overlapped Actors for Abilities
  (if (and (`self.GroundPoundActive`) (`KismetSystemLibrary.DoesImplementInterface` OtherActor "/Game/Forsaken/Characters/BPI_Abilities.BPI_Abilities_C"))
    (bind _returnvalue (`KismetArrayLibrary.Array_AddUnique` (`self.OverlappedActors`) OtherActor))))

(event `self.Sphere.OnComponentEndOverlap`
  (params (OverlappedComponent :type "PrimitiveComponent Object Reference") (OtherActor :type "Actor Object Reference") (OtherComp :type "PrimitiveComponent Object Reference") (OtherBodyIndex :type Integer))
  ;[1 0.5 0] Store Overlapped Actors for Abilities
  (if (and (`self.GroundPoundActive`) (`KismetSystemLibrary.DoesImplementInterface` OtherActor "/Game/Forsaken/Characters/BPI_Abilities.BPI_Abilities_C"))
    (`KismetArrayLibrary.Array_RemoveItem` (`self.OverlappedActors`) OtherActor)))

(fn `UserConstructionScript`)