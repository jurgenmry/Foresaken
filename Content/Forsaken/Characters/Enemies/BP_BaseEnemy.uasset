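; BP_BaseEnemy is an enemy character base for Forsaken that handles death and a pickup drop.
; A Dead event, guarded by DoOnce, plays the death animation on the mesh and disables capsule collision.
; After short delays it spawns a BP_BasePickup at the enemy's location, then destroys the actor.
; BeginPlay only calls its parent, and the overlap and tick events are disabled.
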(event `self.ReceiveBeginPlay`
  (`parent.ReceiveBeginPlay`))

(event `self.Dead`
  (`/Engine/EditorBlueprintResources/StandardMacros.DoOnce` false
    (:`Completed`
      (`SkeletalMeshComponent.PlayAnimation` (`self.Mesh`) (`self.AnimationDeath`) false)
      (`PrimitiveComponent.SetCollisionEnabled` (`self.CapsuleComponent`) "NoCollision")
      (`KismetSystemLibrary.Delay` 1.0)
      (`|SpawnActorFromClass` "/Game/Forsaken/InteractableObjects/BP_BasePickup.BP_BasePickup_C" (`KismetMathLibrary.MakeTransform` (`self.K2_GetActorLocation`)) "AdjustIfPossibleButAlwaysSpawn" "OverrideRootScale" null null)
      (`KismetSystemLibrary.Delay` 3.0)
      (`self.K2_DestroyActor`))))

(event `self.ReceiveDestroyed`)

(fn `UserConstructionScript`
  (`parent.UserConstructionScript`))