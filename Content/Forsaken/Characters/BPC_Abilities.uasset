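; Ability component for Forsaken characters, providing a Dash and a Ground Hit, with parts specific to the Kwang player.
; Dash adds an impulse along last movement input, spawns Niagara FX and hides the mesh until its cooldown ends.
; Ground Hit locks input, launches up then slams down, knocking overlapped characters and objects outward upon landing.
; GroundHitActive is never set true, so that cooldown never blocks; DashSetup is unwired.
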(event `self.ReceiveBeginPlay`
  (bind _returnvalue (`self.GetOwner`))
  ;[1 0 0] Begin Play
  (`|ExecutionSequence`
    (:`then_0`
      (bind _asbp_base_character (cast `/Game/Forsaken/Characters/BP_BaseCharacter` _returnvalue))
      (bind _output_get (set `self.BP Base Character` _asbp_base_character))
      (set `self.Character Movement` (`Character.CharacterMovement` _output_get))
      (set `self.Mesh` (`Character.Mesh` _output_get)))
    (:`then_1`
      (bind _asbp_kwang_player (cast `/Game/Forsaken/Characters/Player/BP_PlayerKwang` _returnvalue))
      (set `self.BP Kwang Player` _asbp_kwang_player))))

(event `Dash`
  (params (DashCooldown :type "Float (double-precision)"))
  (bind _bp_kwang_player (`self.BP Kwang Player`))
  (bind _bp_base_character (`self.BP Base Character`))
  (bind _mesh (`Character.Mesh` _bp_base_character))
  (bind (_returnvalue_roll _returnvalue_pitch _returnvalue_yaw) (`KismetMathLibrary.BreakRotator` (`KismetMathLibrary.MakeRotFromX` (`Actor.GetActorForwardVector` _bp_base_character))))
  ;[0 1 0] DASH
  (if (not (`self.DashActive?`))
    (set `self.DashActive?` true)
    (`CharacterMovementComponent.AddImpulse` (`Character.CharacterMovement` _bp_base_character) (* (`Pawn.GetLastMovementInputVector` _bp_base_character) 10000.0) true)
    (`SceneComponent.SetHiddenInGame` _mesh true false)
    (`NiagaraFunctionLibrary.SpawnSystemAttached` "/Game/NS_Dash_FX.NS_Dash_FX" (`/Game/Forsaken/Characters/Player/BP_PlayerKwang.FXLOC` _bp_kwang_player) "None" (`SceneComponent.K2_GetComponentLocation` (`Actor.RootComponent` _bp_kwang_player)) (`KismetMathLibrary.MakeRotator` 0.0 0.0 _returnvalue_yaw) "KeepWorldPosition" true)
    (`KismetSystemLibrary.Delay` DashCooldown)
    (`SceneComponent.SetHiddenInGame` _mesh false false)
    (set `self.DashActive?` false)))

(event `GroundHit`
  (params (GroundHitCooldown :type "Float (double-precision)"))
  (bind _bp_base_character (`self.BP Base Character`))
  (bind _bp_kwang_player (`self.BP Kwang Player`))
  (bind _bp_base_character_2 (`self.BP Base Character`))
  (bind _returnvalue (`Actor.K2_GetActorLocation` _bp_kwang_player))
  ;[0 1 0] Ground hit
  (if (`self.GroundHitActive?`)
    _
    (elif (not (`/Game/Forsaken/Characters/Player/BP_PlayerKwang.IsAttacking` (`self.BP Kwang Player`)))
      (set `self.GroundHitActive?` false)
      (`Actor.DisableInput` _bp_base_character_2 null)
      (if (not (`NavMovementComponent.IsFalling` (`Character.CharacterMovement` _bp_base_character_2)))
        (`Character.LaunchCharacter` _bp_base_character_2 (`KismetMathLibrary.MakeVector` 0.0 0.0 (`self.LaunchUp`)) true true)
        (`KismetSystemLibrary.Delay` 0.5))
      (`Character.LaunchCharacter` _bp_base_character_2 (0.0 0.0 -1200.0) true true)
      (`KismetSystemLibrary.Delay` 0.2)
      (if (`NavMovementComponent.IsMovingOnGround` (`Character.CharacterMovement` _bp_base_character))
        (for _array_element (`/Game/Forsaken/Characters/Player/BP_PlayerKwang.OverlappedActors` _bp_kwang_player)
          (bind _asbp_base_character (cast `/Game/Forsaken/Characters/BP_BaseCharacter` _array_element)
            (:`then`
              (`Character.LaunchCharacter` _asbp_base_character (* (`KismetMathLibrary.Normal` (- (`Actor.K2_GetActorLocation` _asbp_base_character) _returnvalue)) 3500.0) true true))
            (:`CastFailed`
              (`PrimitiveComponent.AddImpulse` (`Actor.GetComponentByClass` _array_element "/Script/Engine.PrimitiveComponent") (* (`KismetMathLibrary.Normal` (- (`Actor.K2_GetActorLocation` _array_element) _returnvalue)) (`self.ImpulseStrength`)) "None" false))))
        (`Actor.EnableInput` _bp_base_character null)
        (`KismetSystemLibrary.Delay` GroundHitCooldown)
        (set `self.GroundHitActive?` false)))))