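; Health component Blueprint for Forsaken characters that tracks current and maximum health.
; ApplyDamage subtracts damage from current health and returns the new value with a Dead flag once it reaches zero or below.
; AddHealthMax and AddCurrentHealth raise their values and return the results, with no clamping between current and maximum.
; All logic lives in these callable functions; the event graph is empty.
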(event `self.ReceiveBeginPlay`)

(fn `AddCurrentHealth`
  (params (`Health+` :type "Float (double-precision)"))
  (returns (CurrentHealth :type "Float (double-precision)"))
  (bind _output_get (set `self.CurrentHealth` (+ `Health+` (`self.CurrentHealth`))))
  (return _output_get))

(fn `AddHealthMax`
  (params (`Health+` :type "Float (double-precision)"))
  (returns (HealthMax :type "Float (double-precision)"))
  (bind _output_get (set `self.HealthMax` (+ `Health+` (`self.HealthMax`))))
  (return _output_get))

(fn `ApplyDamage`
  (params (Damage :type "Float (double-precision)"))
  (returns (CurrentHealth :type "Float (double-precision)") (`Dead?` :type Boolean))
  (bind _output_get (set `self.CurrentHealth` (- (`self.CurrentHealth`) Damage)))
  (if (<= _output_get 0.0)
    (return _output_get true)
    (else
      (return _output_get false))))