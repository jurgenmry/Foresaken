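; BP_NextLevel is a level-exit trigger actor that moves the player to the next map once the enemy kill quota is met.
; It caches the BP_GMForsaken game mode on BeginPlay.
; When BP_PlayerKwang overlaps its sphere, it compares EnemiesKilled to EnemiesToKill on the game mode and, if they are exactly equal, opens the NextLevel reference.
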(event `self.ReceiveBeginPlay`
  (bind _asbp_gmforsaken (cast `/Game/Forsaken/BP_GMForsaken` (`GameplayStatics.GetGameMode`)))
  (set `self.BP GMForsaken` _asbp_gmforsaken))

(event `self.Sphere.OnComponentBeginOverlap`
  (params (OverlappedComponent :type "PrimitiveComponent Object Reference") (OtherActor :type "Actor Object Reference") (OtherComp :type "PrimitiveComponent Object Reference") (OtherBodyIndex :type Integer) (bFromSweep :type Boolean) (SweepResult :type "HitResult Structure (by ref)"))
  (bind _bp_gmforsaken (`self.BP GMForsaken`))
  (cast `/Game/Forsaken/Characters/Player/BP_PlayerKwang` OtherActor)
  (if (== (`/Game/Forsaken/BP_GMForsaken.EnemiesKilled` _bp_gmforsaken) (`/Game/Forsaken/BP_GMForsaken.EnemiesToKill` _bp_gmforsaken))
    (`GameplayStatics.OpenLevelBySoftObjectPtr` (`self.NextLevel`))))

(fn `UserConstructionScript`)