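; Ability component for the Kwang player character, providing ground hit, dash, rage and ranged attack, each gated by an active flag and a Delay cooldown.
; Ground hit plays a montage with input disabled, then knocks overlapped characters and objects outward.
; Dash teleports along last movement input, using a capsule trace to adjust the destination.
; Rage temporarily multiplies damage, speed and attack rate; ranged attack's projectile is destroyed when cooldown ends.
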(event `self.ReceiveBeginPlay`
  (bind _returnvalue (`self.GetOwner`))
  ;[1 0 0] Begin Play
  (`|ExecutionSequence`
    (:`then_0`
      (bind _asbp_base_character (cast `/Game/Forsaken/Characters/BP_BaseCharacter` _returnvalue))
      (set `self.BP Base Character` _asbp_base_character))
    (:`then_1`
      (bind _asbp_player_kwang (cast `/Game/Forsaken/Characters/Player/BP_PlayerKwang` _returnvalue))
      (set `self.BP Kwang Player` _asbp_player_kwang))))

(event `GroundHit`
  (params (GroundHitCooldown :type "Float (double-precision)"))
  (bind _bp_base_character (`self.BP Base Character`))
  (bind _returnvalue (`Actor.K2_GetActorLocation` _bp_base_character))
  ;[0 1 0] Ground hit
  (if (not (`self.GroundHitActive?`))
    (set `self.GroundHitActive?` true)
    (`Actor.DisableInput` (`self.BP Base Character`) null)
    (`|PlayMontage` (`Character.Mesh` (`self.BP Kwang Player`)) "/Game/Forsaken/Characters/Player/Montage_AbilityPush.Montage_AbilityPush" 1.8
      (:`OnCompleted`
        (for _array_element (`/Game/Forsaken/Characters/Player/BP_PlayerKwang.OverlappedActors` (`self.BP Kwang Player`))
          (bind _asbp_base_character (cast `/Game/Forsaken/Characters/BP_BaseCharacter` _array_element)
            (:`then`
              (`MovementComponent.StopMovementImmediately` (`Character.CharacterMovement` _asbp_base_character))
              (bind (_returnvalue_x _returnvalue_y) (`KismetMathLibrary.BreakVector` (* (`KismetMathLibrary.Normal` (- (`Actor.K2_GetActorLocation` _asbp_base_character) _returnvalue)) 3500.0)))
              (`Character.LaunchCharacter` _asbp_base_character (`KismetMathLibrary.MakeVector` _returnvalue_x _returnvalue_y 50.0) true true))
            (:`CastFailed`
              (`PrimitiveComponent.AddImpulse` (`Actor.GetComponentByClass` _array_element "/Script/Engine.PrimitiveComponent") (* (`KismetMathLibrary.Normal` (- (`Actor.K2_GetActorLocation` _array_element) _returnvalue)) (`self.ImpulseStrength`)) "None" false))))
        (`Actor.EnableInput` _bp_base_character null)
        (`KismetSystemLibrary.Delay` GroundHitCooldown)
        (set `self.GroundHitActive?` false)))))

(event `Dash`
  (params (DashCooldown :type "Float (double-precision)"))
  (bind _bp_base_character (`self.BP Base Character`))
  (bind _returnvalue (`Actor.K2_GetActorLocation` _bp_base_character))
  (bind _capsulecomponent (`Character.CapsuleComponent` _bp_base_character))
  (bind _returnvalue_2 (+ _returnvalue (* (`Pawn.GetLastMovementInputVector` _bp_base_character) 500.0)))
  ;[0 1 0] NEW DASH 2.0
  (if (not (`self.DashActive?`))
    (set `self.DashActive?` true)
    (set `self.HitLocation` _returnvalue_2)
    (bind (_outhits _returnvalue_3) (`KismetSystemLibrary.CapsuleTraceMultiForObjects` _returnvalue _returnvalue_2 (`CapsuleComponent.GetScaledCapsuleRadius` _capsulecomponent) (- (`CapsuleComponent.GetScaledCapsuleHalfHeight` _capsulecomponent) 20.0) (`|MakeArray` "ObjectTypeQuery3" "ObjectTypeQuery1" :!type "EObjectTypeQuery Enum")))
    (if _returnvalue_3
      (for _array_element _outhits
        (bind (_bblockinghit _binitialoverlap _time _distance _location _impactpoint _normal _impactnormal _physmat _hitactor) (`GameplayStatics.BreakHitResult` _array_element))
        (cast `/Game/Forsaken/Characters/BP_BaseCharacter` _hitactor
          (:`CastFailed`
            (set `self.HitLocation` _impactpoint)))))
    (`Actor.K2_SetActorLocation` (`self.BP Base Character`) (`self.HitLocation`) false false)
    (`KismetSystemLibrary.Delay` DashCooldown)
    (set `self.DashActive?` false)))

(event `Rage`
  (params (Duration :type "Float (double-precision)") (Cooldown :type "Float (double-precision)"))
  (bind _charactermovement (`Character.CharacterMovement` (`self.BP Base Character`)))
  (bind _maxwalkspeed (`CharacterMovementComponent.MaxWalkSpeed` _charactermovement))
  ;[0 1 0] Rage
  (if (not (`self.RageActive?`))
    (set `self.RageActive?` true)
    (`|ExecutionSequence`
      (:`then_0`
        (set `self.DamageOriginal` (`/Game/Forsaken/Characters/BP_BaseCharacter.DamageCurrent` (`self.BP Base Character`)))
        (set `/Game/Forsaken/Characters/BP_BaseCharacter.DamageCurrent` (* (`/Game/Forsaken/Characters/BP_BaseCharacter.DamageCurrent` (`self.BP Base Character`)) (`self.DamageMultiplier`)) (`self.BP Base Character`)))
      (:`then_1`
        (set `self.WalkSpeed` _maxwalkspeed)
        (set `CharacterMovementComponent.MaxWalkSpeed` (* (`self.WalkMultiplier`) _maxwalkspeed) _charactermovement))
      (:`then_2`
        (bind _output_get (set `self.AnimPlayRateOriginal` (`/Game/Forsaken/Characters/BP_BaseCharacter.AnimAttackPlayRate` (`self.BP Base Character`))))
        (set `/Game/Forsaken/Characters/BP_BaseCharacter.AnimAttackPlayRate` (* _output_get (`self.AnimPlayRateMultiplier`)) (`self.BP Base Character`)))
      (:`then_3`
        (`KismetSystemLibrary.Delay` Duration)
        (set `/Game/Forsaken/Characters/BP_BaseCharacter.DamageCurrent` (`self.DamageOriginal`) (`self.BP Base Character`))
        (set `CharacterMovementComponent.MaxWalkSpeed` (`self.WalkSpeed`) (`Character.CharacterMovement` (`self.BP Base Character`)))
        (set `/Game/Forsaken/Characters/BP_BaseCharacter.AnimAttackPlayRate` (`self.AnimPlayRateOriginal`) (`self.BP Base Character`)))
      (:`then_4`
        (`KismetSystemLibrary.Delay` Cooldown)
        (set `self.RageActive?` false)))))

(event `RangeAttack`
  (params (Cooldown :type "Float (double-precision)"))
  ;[0 1 0.000306] Range Attack
  (if (not (`self.RangeActive?`))
    (set `self.RangeActive?` true)
    (bind _returnvalue (`|SpawnActorFromClass` "/Game/Forsaken/BP_RangeProjectile.BP_RangeProjectile_C" (`SceneComponent.K2_GetComponentToWorld` (`/Game/Forsaken/Characters/BP_BaseCharacter.SpawnProjectile` (`self.BP Base Character`))) "Undefined" "OverrideRootScale" null null))
    (`KismetSystemLibrary.Delay` Cooldown)
    (set `self.RangeActive?` false)
    (`Actor.K2_DestroyActor` _returnvalue)))

(event `Push`
  (params (GroundHitCooldown :type "Float (double-precision)")))