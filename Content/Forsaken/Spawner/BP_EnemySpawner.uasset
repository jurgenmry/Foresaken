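; BP_EnemySpawner is a wave spawner that sets the Forsaken game mode's kill target to waves times enemies per wave.
; On BeginPlay it caches transforms from SpawnLocations, then after an initial delay spawns waves at a fixed interval until it destroys itself.
; Each enemy gets a random cached transform and random class, though the class roll never selects the Enemy array's last entry.
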(event `self.ReceiveBeginPlay`
  (bind _asbp_gmforsaken (cast `/Game/Forsaken/BP_GMForsaken` (`GameplayStatics.GetGameMode`)))
  (set `/Game/Forsaken/BP_GMForsaken.EnemiesToKill` (* (`self.Waves`) (`self.EnemiesPerWave`)) _asbp_gmforsaken)
  (`self.SetSpawnTransforms`)
  (`KismetSystemLibrary.Delay` (`self.InitialDelay`))
  (if (== (`self.CurrentWaves`) (`self.Waves`)) :!label _label
    (`self.K2_DestroyActor`)
    (else
      (`/Engine/EditorBlueprintResources/StandardMacros.IncrementInt` (`self.CurrentWaves`)
        (:`  `
          (`self.EnemySpawnerLoop`)
          (`KismetSystemLibrary.Delay` (`self.WavesDelay`))
          (goto _label))))))

(fn `EnemySpawnerLoop`
  (locals (TransformIndex :type Integer))
  (for _ (range (`self.EnemiesPerWave`))
    (set `local.TransformIndex` (`KismetMathLibrary.RandomInteger` (`KismetArrayLibrary.Array_Length` (`self.EnemySpawnerArray`))))
    (`|SpawnActorFromClass` (`|GetArrayItem` (`self.Enemy`) (`KismetMathLibrary.RandomInteger` (- (`KismetArrayLibrary.Array_Length` (`self.Enemy`)) 1))) (`|GetArrayItem` (`self.EnemySpawnerArray`) (`local.TransformIndex`)) "AdjustIfPossibleButAlwaysSpawn" "OverrideRootScale" null null)))

(fn `SetSpawnTransforms`
  (for _index (range (`KismetArrayLibrary.Array_Length` (`self.SpawnLocations`)))
    (`KismetArrayLibrary.Array_AddUnique` (`self.EnemySpawnerArray`) (`SceneComponent.K2_GetComponentToWorld` (`Actor.RootComponent` (`|GetArrayItem` (`self.SpawnLocations`) _index))))))

(fn `UserConstructionScript`)