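; AI controller Blueprint for BP_Enemy_1 that runs its behavior tree and feeds the blackboard with patrol and player-sight data.
; On BeginPlay it starts BT_behaviorTree and copies the controlled enemy's PatrolPath looping flag and wait time into the blackboard, along with an initial patrol direction.
; AI Perception updates set the CanSeePlayer key from whether BP_PlayerKwang is successfully sensed.
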(event `self.ReceiveBeginPlay`
  (bind _returnvalue (`AIBlueprintHelperLibrary.GetBlackboard` null))
  (`self.RunBehaviorTree` "/Game/Forsaken/Yorgen_level/Level/AI/BT_behaviorTree.BT_behaviorTree")
  (bind _asbp_enemy_1 (cast `/Game/Forsaken/Characters/Enemies/BP_Enemy_1` (`self.K2_GetPawn`)))
  (bind _output_get (set `self.As BP Enemy 1` _asbp_enemy_1))
  (`BlackboardComponent.SetValueAsBool` (`AIBlueprintHelperLibrary.GetBlackboard` null) "PathLooping" (`/Game/Forsaken/Characters/Enemies/PatrolPath.IsLooping` (`/Game/Forsaken/Characters/Enemies/BP_BaseEnemy.PatrolPath` _output_get)))
  (`BlackboardComponent.SetValueAsInt` _returnvalue "Direction" 1)
  (`BlackboardComponent.SetValueAsFloat` _returnvalue "WaitTime" (`/Game/Forsaken/Characters/Enemies/PatrolPath.WaitTime` (`/Game/Forsaken/Characters/Enemies/BP_BaseEnemy.PatrolPath` (`self.As BP Enemy 1`)))))

(event `self.AIPerception.OnTargetPerceptionUpdated`
  (params (Actor :type "Actor Object Reference") (Stimulus :type "AIStimulus Structure"))
  (cast `/Game/Forsaken/Characters/Player/BP_PlayerKwang` Actor)
  (`BlackboardComponent.SetValueAsBool` (`AIBlueprintHelperLibrary.GetBlackboard` null) "CanSeePlayer" Stimulus_bSuccessfullySensed))

(fn `UserConstructionScript`)