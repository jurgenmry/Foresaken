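; Health component that stores current and maximum health for its owner and exposes functions to change them.
; ApplyDamage subtracts damage from current health, prints the result for debugging and returns whether health has reached zero or below.
; Separate functions add to maximum health, returning the new value, and to current health, with no clamping between the two.
; BeginPlay is empty, so all changes come from external callers.
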(event `self.ReceiveBeginPlay`)

(fn `AddCurrentHealth`
  (params (`Health+` :type "Float (double-precision)"))
  (set `self.Health Current` (+ `Health+` (`self.Health Current`)))
  (return))

(fn `AddHealthMax`
  (params (`Health+` :type "Float (double-precision)"))
  (returns (HealthMax :type "Float (double-precision)"))
  (bind _output_get (set `self.Health Max` (+ `Health+` (`self.Health Max`))))
  (return _output_get))

(fn `ApplyDamage`
  (params (Damage :type "Float (double-precision)"))
  (returns (`Dead?` :type Boolean))
  (bind _output_get (set `self.Health Current` (- (`self.Health Current`) Damage)))
  (`KismetSystemLibrary.PrintString` (`KismetStringLibrary.Conv_DoubleToString` _output_get))
  (if (<= _output_get 0.0)
    (return true)
    (else
      (return false))))