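; BP_Door is a level exit door in Forsaken that opens once the required enemies are killed and leads to another level.
; An Enter overlap by BP_PlayerKwang prints and compares the BP_GMForsaken kill counts, then plays a timeline lowering the door on a match.
; Each update lerps from the current Z rather than a stored start, so movement accumulates.
; An Exit overlap reverses the timeline and immediately opens the referenced level.
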(event `self.ReceiveBeginPlay`
  (bind _asbp_gmforsaken (cast `/Game/Forsaken/BP_GMForsaken` (`GameplayStatics.GetGameMode`)))
  (set `self.BP GMForsaken` _asbp_gmforsaken))

(event `OpenDoor`
  (bind (_returnvalue_x _returnvalue_y _returnvalue_z) (`KismetMathLibrary.BreakVector` (`self.K2_GetActorLocation`)))
  (bind (_direction _newtrack_0) (`Timeline|Open/Close` :!label _label)
    (:`Update`
      (`self.K2_SetActorLocation` (`KismetMathLibrary.MakeVector` _returnvalue_x _returnvalue_y (`KismetMathLibrary.Lerp` _returnvalue_z (- _returnvalue_z 45.0) _newtrack_0))))))

(event `CloseDoor`
  (goto _label :!via `Reverse`))

(event `self.Enter.OnComponentBeginOverlap`
  (params (OverlappedComponent :type "PrimitiveComponent Object Reference") (OtherActor :type "Actor Object Reference") (OtherComp :type "PrimitiveComponent Object Reference") (OtherBodyIndex :type Integer) (bFromSweep :type Boolean) (SweepResult :type "HitResult Structure (by ref)"))
  (bind _bp_gmforsaken (`self.BP GMForsaken`))
  (bind _enemieskilled (`/Game/Forsaken/BP_GMForsaken.EnemiesKilled` _bp_gmforsaken))
  (bind _enemiestokill (`/Game/Forsaken/BP_GMForsaken.EnemiesToKill` _bp_gmforsaken))
  (cast `/Game/Forsaken/Characters/Player/BP_PlayerKwang` OtherActor)
  (`KismetSystemLibrary.PrintString` (`KismetStringLibrary.Concat_StrStr` (`KismetStringLibrary.Conv_IntToString` _enemieskilled) "   Killed"))
  (`KismetSystemLibrary.PrintString` (`KismetStringLibrary.Concat_StrStr` (`KismetStringLibrary.Conv_IntToString` _enemiestokill) "   TO KILL"))
  (if (== _enemieskilled _enemiestokill)
    (`self.OpenDoor`)))

(event `self.Exit.OnComponentBeginOverlap`
  (params (OverlappedComponent :type "PrimitiveComponent Object Reference") (OtherActor :type "Actor Object Reference") (OtherComp :type "PrimitiveComponent Object Reference") (OtherBodyIndex :type Integer) (bFromSweep :type Boolean) (SweepResult :type "HitResult Structure (by ref)"))
  (cast `/Game/Forsaken/Characters/Player/BP_PlayerKwang` OtherActor)
  (`self.CloseDoor`)
  (`GameplayStatics.OpenLevelBySoftObjectPtr` (`self.Level`)))

(fn `UserConstructionScript`)