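; BP_EnemySpawner is a wave-based spawner actor that places random enemies at six preset spawn points.
; On BeginPlay it caches the world transforms of those points, then starts a delay-driven wave loop after a short initial pause.
; Each wave spawns a set number of enemies, picking both class and location at random.
; The actor destroys itself once the configured wave count is reached.
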(event `self.ReceiveBeginPlay`
  (set `self.EnemySpawnerArray` (`|MakeArray` (`SceneComponent.K2_GetComponentToWorld` (`self.EnemySpawner`)) (`SceneComponent.K2_GetComponentToWorld` (`self.EnemySpawner1`)) (`SceneComponent.K2_GetComponentToWorld` (`self.EnemySpawner2`)) (`SceneComponent.K2_GetComponentToWorld` (`self.EnemySpawner3`)) (`SceneComponent.K2_GetComponentToWorld` (`self.EnemySpawner4`)) (`SceneComponent.K2_GetComponentToWorld` (`self.EnemySpawner5`))))
  (`KismetSystemLibrary.Delay` 5.0)
  (if (== (`self.CurrentWaves`) (`self.Waves`)) :!label _label
    (`self.K2_DestroyActor`)
    (else
      (`/Engine/EditorBlueprintResources/StandardMacros.IncrementInt` (`self.CurrentWaves`)
        (:`  `
          (`self.EnemySpawnerLoop`)
          (`KismetSystemLibrary.Delay` (`self.SpawnDelay`))
          (goto _label))))))

(fn `EnemySpawnerLoop`
  (for _ (range (`self.NumberOfEnemies`))
    (`|SpawnActorFromClass` (`|GetArrayItem` (`self.Enemy`) (`KismetMathLibrary.RandomInteger` (`KismetArrayLibrary.Array_Length` (`self.Enemy`)))) (`|GetArrayItem` (`self.EnemySpawnerArray`) (`KismetMathLibrary.RandomInteger` (`KismetArrayLibrary.Array_Length` (`self.EnemySpawnerArray`)))) "Undefined" "OverrideRootScale" null null)))

(fn `UserConstructionScript`)