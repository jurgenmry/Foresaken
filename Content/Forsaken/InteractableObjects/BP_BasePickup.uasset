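; Base pickup actor that automatically homes in on the first player character and reports its pickup type when destroyed.
; One second after spawning, a timeline lerps it from its current location toward the player's live position on X and Y, keeping its height.
; It destroys itself when the timeline finishes, with no overlap check.
; The Destroyed event then passes PickUpType to BP_PlayerState through CallOnPickedUp.
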(event `self.ReceiveBeginPlay`
  (`KismetSystemLibrary.Delay` 1.0)
  (bind (_direction _lerp_2sec) (`Timeline|Movement`)
    (:`Update`
      (`self.SetLocation` (`GameplayStatics.GetPlayerCharacter` 0) _lerp_2sec))
    (:`Finished`
      (`self.K2_DestroyActor`))))

(event `self.ReceiveDestroyed`
  (bind _asbp_player_state (cast `/Game/Forsaken/BP_PlayerState` (`Pawn.PlayerState` (`GameplayStatics.GetPlayerCharacter` 0)))
    (:`then`
      (`/Game/Forsaken/BP_PlayerState.OnPickedUp` _asbp_player_state (`self.PickUpType`)))
    (:`CastFailed`
      (`KismetSystemLibrary.PrintString` "fail"))))

(fn `SetLocation`
  (params (ActorToMove :type "Actor Object Reference") (Alpha :type "Float (double-precision)"))
  (bind (_returnvalue_x _returnvalue_y _returnvalue_z) (`KismetMathLibrary.BreakVector` (`self.K2_GetActorLocation`)))
  (bind (_returnvalue_x_2 _returnvalue_y_2) (`KismetMathLibrary.BreakVector` (`self.K2_GetActorLocation` ActorToMove)))
  (`self.K2_SetActorLocation` (`KismetMathLibrary.MakeVector` (`KismetMathLibrary.Lerp` _returnvalue_x _returnvalue_x_2 Alpha) (`KismetMathLibrary.Lerp` _returnvalue_y _returnvalue_y_2 Alpha) _returnvalue_z)))

(fn `UserConstructionScript`)